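; Ball actor for a brick-breaker game that bounces around the level and notifies what it hits.
; During one game state, Tick sweeps it in XY by Direction times Speed, without delta-time scaling, and reflects Direction off the impact normal.
; Paddle hits skew the bounce by paddle input and an X bias; other hit actors receive HitByBall through BallHitInterface.
; The game mode's start-playing event resets ball and paddle positions.
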(event Custom|BallStartPlaying
  (CallFunction|ResetBallPosition))

(event EventBeginPlay
  (bind _asbrick_game_mode (Utilities|Casting|CastToBrickGameMode (Game|GetGameMode)))
  (EventDispatchers|BindEventtoStartPlaying _asbrick_game_mode (delegate Custom|BallStartPlaying)))

(event Collision|EventActorBeginOverlap
  (params (OtherActor :type Actor%20Object%20Reference)))

(event EventTick
  (params (DeltaSeconds :type Float%20%28single-precision%29))
  (bind _asbrick_game_mode (Utilities|Casting|CastToBrickGameMode (Game|GetGameMode)))
  (if (Utilities|Enum|Equal(Enum) (Variables|/Game/Blueprints/GameMode/BrickGameMode.BrickGameMode_C|GetStateOfGame _asbrick_game_mode) "NewEnumerator6")
    (bind _sweephitresult (Transformation|AddActorWorldOffset (Math|Vector|MakeVector (.X (Math|Vector|BreakVector (* (Variables|Default|GetDirection) (Variables|Default|Getspeed)))) (.Y (Math|Vector|BreakVector (* (Variables|Default|GetDirection) (Variables|Default|Getspeed)))) 0.0) true))
    (bind _aspaddle (Utilities|Casting|CastToPaddle (.HitActor (Collision|BreakHitResult _sweephitresult)))
      (:then
        (Variables|Default|SetDirection (Math|Vector|Normalize (Math|Vector|MakeVector (+ (Variables|Default|GetMinX) (.x (Math|Vector|Normalize (Math|Vector|MakeVector (.X (Math|Vector|BreakVector (Math|Vector|GetReflectionVector (Variables|Default|GetDirection) (.ImpactNormal (Collision|BreakHitResult _sweephitresult))))) (+ (* (Variables|/Game/Blueprints/Pawns/Paddle.Paddle_C|GetAxisValue _aspaddle) 5.0) (.Y (Math|Vector|BreakVector (Math|Vector|GetReflectionVector (Variables|Default|GetDirection) (.ImpactNormal (Collision|BreakHitResult _sweephitresult)))))) (.Z (Math|Vector|BreakVector (Math|Vector|GetReflectionVector (Variables|Default|GetDirection) (.ImpactNormal (Collision|BreakHitResult _sweephitresult))))))))) (.y (Math|Vector|Normalize (Math|Vector|MakeVector (.X (Math|Vector|BreakVector (Math|Vector|GetReflectionVector (Variables|Default|GetDirection) (.ImpactNormal (Collision|BreakHitResult _sweephitresult))))) (+ (* (Variables|/Game/Blueprints/Pawns/Paddle.Paddle_C|GetAxisValue _aspaddle) 5.0) (.Y (Math|Vector|BreakVector (Math|Vector|GetReflectionVector (Variables|Default|GetDirection) (.ImpactNormal (Collision|BreakHitResult _sweephitresult)))))) (.Z (Math|Vector|BreakVector (Math|Vector|GetReflectionVector (Variables|Default|GetDirection) (.ImpactNormal (Collision|BreakHitResult _sweephitresult)))))))) (.z (Math|Vector|Normalize (Math|Vector|MakeVector (.X (Math|Vector|BreakVector (Math|Vector|GetReflectionVector (Variables|Default|GetDirection) (.ImpactNormal (Collision|BreakHitResult _sweephitresult))))) (+ (* (Variables|/Game/Blueprints/Pawns/Paddle.Paddle_C|GetAxisValue _aspaddle) 5.0) (.Y (Math|Vector|BreakVector (Math|Vector|GetReflectionVector (Variables|Default|GetDirection) (.ImpactNormal (Collision|BreakHitResult _sweephitresult)))))) (.Z (Math|Vector|BreakVector (Math|Vector|GetReflectionVector (Variables|Default|GetDirection) (.ImpactNormal (Collision|BreakHitResult _sweephitresult))))))))))))
      (:CastFailed
        (Variables|Default|SetDirection (Math|Vector|GetReflectionVector (Variables|Default|GetDirection) (.ImpactNormal (Collision|BreakHitResult _sweephitresult))))
        (if (Utilities|DoesObjectImplementInterface (.HitActor (Collision|BreakHitResult _sweephitresult)) "/Game/Blueprints/Interfaces/BallHitInterface.BallHitInterface_C")
          (Class|BallHitInterface|HitbyBall(Message) (.HitActor (Collision|BreakHitResult _sweephitresult))))))))

(fn ConstructionScript)

(fn ResetBallPosition
  (Transformation|SetActorLocation "-200.000000, 0,1.000000" false false)
  (Variables|Default|SetDirection (Math|Vector|Normalize (Math|Vector|MakeVector 1.0 0.0 0.0) 0.01))
  (bind _aspaddle (Utilities|Casting|CastToPaddle (Game|Player|GetPlayerPawn 0)))
  (Transformation|SetActorLocation _aspaddle "-400.000000, 0,2.062599" false false))