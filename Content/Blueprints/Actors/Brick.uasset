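; Breakable brick actor that loses a hit point each time the ball hits it, in a brick-breaker style game.
; Its material color follows remaining hit points, and a widget component shows a BrickNumber widget given a reference to the brick.
; Every hit plays a sound and adds to the GameInstance score; the final hit also decrements the GameMode brick count and destroys the actor.
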(event EventBeginPlay
  (CallFunction|SelectBrickColor (Variables|Default|GetHitPoints))
  (bind _returnvalue (UserInterface|CreateWidget "/Game/HUD/Widgets/BrickNumber.BrickNumber_C"))
  (Variables|/Game/HUD/Widgets/BrickNumber.BrickNumber_C|SetREF_Brick _returnvalue self)
  (UserInterface|SetWidget (Variables|Default|GetNumberComponentWidget) _returnvalue))

(event EventHitbyBall
  (CallFunction|DecrementHitPoints))

(fn ConstructionScript)

(fn DecrementHitPoints
  (bind _returnvalue (Game|GetGameInstance))
  (if (<= (- (Variables|Default|GetHitPoints) 1) 0)
    (Audio|PlaySound2D "/Game/Interface_And_Item_Sounds/Cues/Coins_02_Cue.Coins_02_Cue" 1.0 1.0 0.0 0 0)
    (bind _asbrick_game_mode (Utilities|Casting|CastToBrickGameMode (Game|GetGameMode)))
    (Default|DecrementBrickCount _asbrick_game_mode)
    (bind _asbrick_game_instance (Utilities|Casting|CastToBrickGameInstance _returnvalue))
    (Math|Integer|IncrementInt (Variables|/Game/Blueprints/GameInstances/BrickGameInstance.BrickGameInstance_C|GetPlayerScore _asbrick_game_instance)
      (:%20%20
        (Actor|DestroyActor)))
    (else
      (bind _result (Math|Integer|DecrementInt (Variables|Default|GetHitPoints))
        (:%20%20
          (CallFunction|SelectBrickColor _result)
          (Audio|PlaySound2D "/Game/Interface_And_Item_Sounds/Cues/Coins_01_Cue.Coins_01_Cue" 1.0 1.0 0.0 0 0)
          (bind _asbrick_game_instance_2 (Utilities|Casting|CastToBrickGameInstance _returnvalue))
          (Math|Integer|IncrementInt (Variables|/Game/Blueprints/GameInstances/BrickGameInstance.BrickGameInstance_C|GetPlayerScore _asbrick_game_instance_2)))))))

(fn SelectBrickColor
  (params (Points :type Integer))
  (switch int Points
    (:0
      _)
    (:1
      (Variables|Default|SetColor "/Game/Materials/Instances/MI_Ball_Red.MI_Ball_Red"))
    (:2
      (Variables|Default|SetColor "/Game/Materials/Instances/MI_Ball_Green.MI_Ball_Green"))
    (:3
      (Variables|Default|SetColor "/Game/Materials/Instances/MI_Ball_Blue.MI_Ball_Blue"))
    (:4
      (Variables|Default|SetColor "/Game/Materials/Instances/MI_Ball_Yellow.MI_Ball_Yellow")))
  (Rendering|Material|SetMaterial (Variables|Default|GetBrickMesh) 0 (Variables|Default|GetColor))
  (return))