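; Brick actor for a brick-breaker game that loses a hit point each time the ball hits it and is destroyed when none remain.
; Its mesh material is chosen from the remaining hit points (red, green or blue) at BeginPlay and after each non-fatal hit.
; On BeginPlay it also creates a BrickNumber widget, passes it a reference to itself and assigns it to its widget component.
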(event EventBeginPlay
  (CallFunction|SelectBrickColor (Variables|Default|GetHitPoints))
  (bind _returnvalue (UserInterface|CreateWidget "/Game/HUD/BrickNumber.BrickNumber_C"))
  (Variables|/Game/HUD/BrickNumber.BrickNumber_C|SetREF_Brick _returnvalue self)
  (UserInterface|SetWidget (Variables|Default|GetNumberComponentWidget) _returnvalue))

(event EventHitbyBall
  (CallFunction|DecrementHitPoints))

(fn ConstructionScript)

(fn DecrementHitPoints
  (if (<= (- (Variables|Default|GetHitPoints) 1) 0)
    (Actor|DestroyActor)
    (else
      (bind _result (Math|Integer|DecrementInt (Variables|Default|GetHitPoints))
        (:%20%20
          (CallFunction|SelectBrickColor _result))))))

(fn SelectBrickColor
  (params (Points :type Integer))
  (switch int Points
    (:0
      _)
    (:1
      (Variables|Default|SetColor "/Game/Materials/Instances/MI_Ball_Red.MI_Ball_Red"))
    (:2
      (Variables|Default|SetColor "/Game/Materials/Instances/MI_Ball_Green.MI_Ball_Green"))
    (:3
      (Variables|Default|SetColor "/Game/Materials/Instances/MI_Ball_Blue.MI_Ball_Blue")))
  (Rendering|Material|SetMaterial (Variables|Default|GetBrickMesh) 0 (Variables|Default|GetColor))
  (return))