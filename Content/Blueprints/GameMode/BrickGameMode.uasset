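; Game mode for a brick game that holds the match state and switches it through SetGameState.
; Countdown resets a timer that Tick runs down, updating a 3-2-1 Count before switching to Playing, which fires the StartPlaying dispatcher.
; Oops returns to Ready after a short delay, while Ready, Game Over and Level Completed only store the state.
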(event Custom|SetGameState
  (params (StateOfGame :type StateOfGame%20Enum :default "NewEnumerator1"))
  (switch Utilities|FlowControl|Switch|SwitchonStateOfGame StateOfGame
    (:NewEnumerator1
      (Variables|Default|SetStateOfGame StateOfGame :!label _label))
    (:NewEnumerator2
      (Variables|Default|SetCountdown 3.0)
      (Variables|Default|SetStateOfGame "NewEnumerator2"))
    (:NewEnumerator3
      (Variables|Default|SetStateOfGame "NewEnumerator3")
      (Utilities|FlowControl|Delay 1.5)
      (CallFunction|SetGameState "NewEnumerator1"))
    (:NewEnumerator4
      (goto _label))
    (:NewEnumerator5
      (goto _label))
    (:NewEnumerator6
      (Default|CallStartPlaying)
      (Variables|Default|SetStateOfGame "NewEnumerator6"))))

(event EventBeginPlay
  (Variables|Default|SetStateOfGame "NewEnumerator1"))

(event EventTick
  (params (DeltaSeconds :type Float%20%28single-precision%29))
  (if (Utilities|Enum|Equal(Enum) (Variables|Default|GetStateOfGame) "NewEnumerator2")
    (bind _output_get (Variables|Default|SetCountdown (- (Variables|Default|GetCountdown) DeltaSeconds)))
    (if (>= _output_get 2.0)
      (Variables|Default|SetCount 3)
      (elif (>= _output_get 1.0)
        (Variables|Default|SetCount 2)
        (elif (>= _output_get 0.0)
          (Variables|Default|SetCount 1)
          (else
            (CallFunction|SetGameState "NewEnumerator6")))))))

(fn ConstructionScript)