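; Paddle pawn for a brick-breaker game that the player slides sideways with the mouse.
; On BeginPlay it lowers its mesh in world Z, then maps the MouseLeftRight axis to swept Y offsets only while BrickGameMode is in one specific game state.
; Movement is per input event, with no delta-time scaling.
; It also holds the BallLives count, which DecrementLives reduces without going below zero.
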(event EventBeginPlay
  (bind _paddlemesh (Variables|Default|GetPaddleMesh))
  (bind _returnvalue (Transformation|GetWorldLocation _paddlemesh))
  (Transformation|SetWorldLocation _paddlemesh (Math|Vector|MakeVector (.x _returnvalue) (.y _returnvalue) (- (.z _returnvalue) 9e+01)) false false))

(event Input|AxisEvents|InputAxisMouseLeftRight
  (params (AxisValue :type Float%20%28single-precision%29))
  (bind _asbrick_game_mode (Utilities|Casting|CastToBrickGameMode (Game|GetGameMode)))
  (if (Utilities|Enum|Equal(Enum) (Variables|/Game/Blueprints/GameMode/BrickGameMode.BrickGameMode_C|GetStateOfGame _asbrick_game_mode) "NewEnumerator6")
    (Variables|Default|SetAxisValue AxisValue)
    (Transformation|AddActorWorldOffset (Math|Vector|MakeVector 0.0 (* AxisValue 25.0) 0.0) true)))

(fn ConstructionScript)

(fn DecrementLives
  (if (not (< (- (Variables|Default|GetBallLives) 1) 0))
    (Math|Integer|DecrementInt (Variables|Default|GetBallLives))))